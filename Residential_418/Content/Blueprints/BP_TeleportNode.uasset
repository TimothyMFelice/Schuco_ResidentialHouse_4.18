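; BP_TeleportNode is a VR teleport destination that moves the player pawn to a set location relative to the node.
; It holds a BP_TeleportPreview child actor, caches it on BeginPlay and hides the component; SetupNode colors the preview blue.
; TeleportPlayer adds the horizontal pawn-to-camera offset so the headset, rather than the pawn origin, lands on the target.
; The logic to hide the preview's chaperone bounds is disconnected.
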(event EventBeginPlay
  ;[1 1 1] Get the actual teleport preview
  (bind _asbp_teleport_preview (Utilities|Casting|CastToBP_TeleportPreview (Variables|/Script/Engine.ChildActorComponent|GetChildActor (Variables|Default|GetTeleportPreview))))
  (Variables|Default|SetTeleportPreviewObject _asbp_teleport_preview)
  (Rendering|SetVisibility (Variables|Default|GetTeleportPreview) false false))

(fn ConstructionScript)

(fn SetupNode
  ;[1 1 1] Default color to blue
  (bind _asbp_teleport_preview (Utilities|Casting|CastToBP_TeleportPreview (Variables|/Script/Engine.ChildActorComponent|GetChildActor (Variables|Default|GetTeleportPreview))))
  (Default|SetColor _asbp_teleport_preview "(R=0.124772,G=0.597202,B=1.000000,A=1.000000)"))

(fn TeleportPlayer
  (bind _returnvalue (Game|GetPlayerCameraManager 0))
  (bind _returnvalue_2 (Game|Player|GetPlayerPawn 0))
  (bind _returnvalue_3 (Camera|GetCameraLocation _returnvalue))
  (bind _returnvalue_4 (Transformation|GetActorLocation _returnvalue_2))
  (bind _returnvalue_5 (- _returnvalue_4 _returnvalue_3))
  (Transformation|SetActorLocation (Game|Player|GetPlayerPawn 0) (+ (+ (Transformation|GetActorLocation) (Variables|Default|GetTeleportToLocation)) (Math|Vector|MakeVector (.x _returnvalue_5) (.y _returnvalue_5) 0.0)) false false))