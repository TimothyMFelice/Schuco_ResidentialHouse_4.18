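; VR-grabbable pivot for the AWS75 unit that swings its moveable part in yaw between min and max limits.
; Pickup requires a controller grab sphere overlapping the handle trigger, then each tick turns the part to follow the hand's local angle minus the initial grab offset.
; On release, a gated tick coasts it analytically from release velocity with friction until it stops or nears a limit.
; Pickup also switches the forced LOD.
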(event Custom|OnDrag
  (bind _returnvalue (Transformation|GetActorTransform))
  (bind _moveable (Variables|Default|GetMoveable))
  (bind _currentgrabsphere (Variables|Default|GetCurrentGrabSphere))
  (bind _returnvalue_2 (Transformation|GetWorldLocation _currentgrabsphere))
  (bind _relativelocation (Variables|/Script/Engine.SceneComponent|GetRelativeLocation _moveable))
  (bind _returnvalue_3 (Math|Transform|InverseTransformLocation _returnvalue _returnvalue_2))
  (bind _returnvalue_4 (- _returnvalue_3 _relativelocation))
  ;[1 1 1] On Drag
  (if (Variables|Vars|GetDragging)
    (Variables|Vars|SetPreviousRotation (Variables|/Script/Engine.SceneComponent|GetRelativeRotation (Variables|Default|GetMoveable)))
    (Transformation|SetRelativeRotation (Variables|Default|GetMoveable) (Math|Rotator|MakeRotator 0.0 0.0 (Math|Float|ClampAngle (- (Class|KismetMathLibrary|DegAtan2 (.y _returnvalue_4) (.x _returnvalue_4)) (Variables|Vars|GetInitialGrabOffset)) (Variables|Vars|GetMinYaw) (Variables|Vars|GetMaxYaw))) false false)))

(event EventPickup
  (params (AttachTo :type Scene%20Component%20Object%20Reference))
  (bind (_isoverlapping _grabsphere) (CallFunction|IsHandOverlapping))
  (bind _returnvalue (Transformation|GetActorTransform))
  (bind _moveable (Variables|Default|GetMoveable))
  (bind _returnvalue_2 (Transformation|GetWorldLocation _grabsphere))
  (bind _relativelocation (Variables|/Script/Engine.SceneComponent|GetRelativeLocation _moveable))
  (bind _returnvalue_3 (Math|Transform|InverseTransformLocation _returnvalue _returnvalue_2))
  (bind _returnvalue_4 (- _returnvalue_3 _relativelocation))
  ;[1 1 1] Grabbed
  (if _isoverlapping
    (Rendering|LOD|SetForcedLodModel (Variables|Default|GetAWS75_Moveable) 1)
    (Variables|Vars|SetInitialGrabOffset (- (Class|KismetMathLibrary|DegAtan2 (.y _returnvalue_4) (.x _returnvalue_4)) (.yaw (Variables|/Script/Engine.SceneComponent|GetRelativeRotation _moveable))))
    (CallFunction|StopSimulatePhysics)
    (Variables|Vars|SetDragging true)))

(event EventBeginPlay
  ;[1 1 1] Setup Initial Vars
  (Variables|Vars|SetInitialRotation (Variables|/Script/Engine.SceneComponent|GetRelativeRotation (Variables|Default|GetMoveable)))
  (Rendering|LOD|SetForcedLodModel (Variables|Default|GetAWS75_Moveable) 2))

(event EventDropNear
  ;[1 1 1] Drop
  (if (Variables|Vars|GetDragging)
    (CallFunction|StartSimulatePhysics (/ (- (.yaw (Variables|/Script/Engine.SceneComponent|GetRelativeRotation (Variables|Default|GetMoveable))) (.yaw (Variables|Vars|GetPreviousRotation))) (Utilities|Time|GetWorldDeltaSeconds)))
    (Variables|Vars|SetDragging false)))

(event Custom|StartSimulatePhysics
  (params (InitialYawVelocity :type Float%20%28single-precision%29))
  (Variables|Vars|SetInitialYawVelocity InitialYawVelocity)
  (Variables|Vars|SetPhysicsInitialYawAngle (.yaw (Variables|/Script/Engine.SceneComponent|GetRelativeRotation (Variables|Default|GetMoveable))))
  (Variables|Vars|SetTimeSinceLetGo 0.0)
  (Utilities|FlowControl|Gate true) ; enters at Open
)

(event Custom|StopSimulatePhysics
  (Utilities|FlowControl|Gate true) ; enters at Close
)

(event EventTick
  (params (DeltaSeconds :type Float%20%28single-precision%29))
  (Utilities|FlowControl|Sequence
    (:then_0
      (Utilities|FlowControl|Gate true
        (:Exit
          (Variables|Vars|SetTimeSinceLetGo (+ DeltaSeconds (Variables|Vars|GetTimeSinceLetGo)))
          (if (|StopPhysicsCheck)
            (CallFunction|StopSimulatePhysics)
            (else
              (Transformation|SetRelativeRotation (Variables|Default|GetMoveable) (Math|Rotator|MakeRotator 0.0 0.0 (|Physics)) false false))))))
    (:then_1
      (CallFunction|OnDrag))))

(fn ConstructionScript)

(fn IsHandOverlapping
  (bind _handletrigger (Variables|Default|GetHandleTrigger))
  (bind _vrpawn (Variables|Settings|GetVRPawn))
  (bind _rightcontroller (Variables|/Game/VirtualRealityBP/Blueprints/MotionControllerPawn.MotionControllerPawn_C|GetRightController _vrpawn))
  (bind _leftcontroller (Variables|/Game/VirtualRealityBP/Blueprints/MotionControllerPawn.MotionControllerPawn_C|GetLeftController _vrpawn))
  (bind _grabsphere (Variables|/Game/VirtualRealityBP/Blueprints/BP_MotionController.BP_MotionController_C|GetGrabSphere _rightcontroller))
  (bind _grabsphere_2 (Variables|/Game/VirtualRealityBP/Blueprints/BP_MotionController.BP_MotionController_C|GetGrabSphere _leftcontroller))
  (if (Class|PrimitiveComponent|IsOverlappingComponent _grabsphere _handletrigger)
    (bind _output_get (Variables|Default|SetCurrentGrabSphere _grabsphere))
    (bind _output_get_2 (Variables|Default|SetIsOverlapping true))
    (return _output_get_2 _output_get)
    (elif (Class|PrimitiveComponent|IsOverlappingComponent _handletrigger _grabsphere_2)
      (bind _output_get_3 (Variables|Default|SetCurrentGrabSphere _grabsphere_2))
      (bind _output_get_4 (Variables|Default|SetIsOverlapping true))
      (return _output_get_4 _output_get_3)
      (else
        (Variables|Default|SetCurrentGrabSphere 0)
        (Variables|Default|SetIsOverlapping false)
        (return false 0)))))